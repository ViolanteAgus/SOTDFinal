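; Player character for a side-scrolling game with jumping, coin collection and a quit action, driven by Enhanced Input.
; Movement follows world X only, and the acceleration sign snaps control yaw to 0 or 180 to face the travel direction.
; The increased and decreased "gravity" actions temporarily raise or lower jump velocity rather than altering gravity, restoring it on completion.
; ObtenerMonedas updates the coin count and prints it on screen.
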(event `self.ReceiveBeginPlay`
  (bind _asplayer_controller (cast `PlayerController` (`self.GetController`)))
  (`EnhancedInputSubsystemInterface.AddMappingContext` (pcsubsystem `EnhancedInputLocalPlayerSubsystem` _asplayer_controller) "/Game/Inputs/IMC_SOTD.IMC_SOTD" 0 (struct)))

(event `EnhancedInput|/Game/Inputs/IA_Jump`
  (params (ActionValue :type "Float (double-precision)") (ElapsedSeconds :type "Float (double-precision)") (TriggeredSeconds :type "Float (double-precision)") (InputAction :type "InputAction Object Reference" :default "/Game/Inputs/IA_Jump.IA_Jump"))
  (:`Triggered`
    (set `self.JumpMaxHoldTime` 0.2)
    (`self.Jump`)))

(event `EnhancedInput|/Game/Inputs/IA_Movimiento`
  (params (ActionValue :type "Float (double-precision)") (ElapsedSeconds :type "Float (double-precision)") (TriggeredSeconds :type "Float (double-precision)") (InputAction :type "InputAction Object Reference" :default "/Game/Inputs/IA_Movimiento.IA_Movimiento"))
  (bind _returnvalue (`self.GetController`))
  (bind _returnvalue_x (`KismetMathLibrary.BreakVector` (`CharacterMovementComponent.GetCurrentAcceleration` (`self.CharacterMovement`))))
  (:`Triggered`
    (`self.AddMovementInput` (1.0 0.0 0.0) ActionValue)
    (`/Engine/EditorBlueprintResources/StandardMacros.CompareFloat` _returnvalue_x
      (:`>`
        (`Controller.SetControlRotation` _returnvalue (`KismetMathLibrary.MakeRotator` 0.0)))
      (:`<`
        (`Controller.SetControlRotation` _returnvalue (`KismetMathLibrary.MakeRotator` 0.0 0.0 180.0))))))

(event `EnhancedInput|/Game/Inputs/IA_GravedadAumentada`
  (params (ActionValue :type "Float (double-precision)") (ElapsedSeconds :type "Float (double-precision)") (TriggeredSeconds :type "Float (double-precision)") (InputAction :type "InputAction Object Reference" :default "/Game/Inputs/IA_GravedadAumentada.IA_GravedadAumentada"))
  (:`Triggered`
    (set `CharacterMovementComponent.JumpZVelocity` 480.0 (`self.CharacterMovement`)))
  (:`Completed`
    (set `CharacterMovementComponent.JumpZVelocity` 220.0 (`self.CharacterMovement`))))

(event `/Game/Interfaces/BPI_Recolectar.ObtenerMonedas`
  (params (Monedas :type Integer))
  (bind _output_get (set `self.Monedas` (+ Monedas (`self.Monedas`))))
  (`KismetSystemLibrary.PrintString` (`KismetStringLibrary.Concat_StrStr` "Agarraste " (`KismetStringLibrary.Conv_IntToString` _output_get) " Monedas") true true (struct :`G` 0.66 :`B` 1.0 :`A` 1.0) 5.0))

(event `EnhancedInput|/Game/Inputs/IA_GravedadDisminuida`
  (params (ActionValue :type "Float (double-precision)") (ElapsedSeconds :type "Float (double-precision)") (TriggeredSeconds :type "Float (double-precision)") (InputAction :type "InputAction Object Reference" :default "/Game/Inputs/IA_GravedadDisminuida.IA_GravedadDisminuida"))
  (:`Triggered`
    (set `CharacterMovementComponent.JumpZVelocity` 100.0 (`self.CharacterMovement`)))
  (:`Completed`
    (set `CharacterMovementComponent.JumpZVelocity` 220.0 (`self.CharacterMovement`))))

(event `EnhancedInput|/Game/Inputs/IA_QuitGame`
  (params (ActionValue :type Boolean) (ElapsedSeconds :type "Float (double-precision)") (TriggeredSeconds :type "Float (double-precision)") (InputAction :type "InputAction Object Reference" :default "/Game/Inputs/IA_QuitGame.IA_QuitGame"))
  (:`Triggered`
    (`KismetSystemLibrary.QuitGame` null "Quit")))

(fn `UserConstructionScript`)